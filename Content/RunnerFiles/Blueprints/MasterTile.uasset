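; Endless-runner track tile that spawns obstacles on three lanes, skipping tiles near the start (cube X below 1500).
; Each lane draws weighted-random from the Obstacles class-to-weight map, tracking spawns in ObstaclesList.
; When the player capsule overlaps Box, the game mode spawns another tile; 0.5 seconds later it adds points and the tile destroys itself and its obstacles.
; A player speed-up branch is present but never runs.
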(event `self.ReceiveBeginPlay`
  (bind _returnvalue_x (`KismetMathLibrary.BreakVector` (`SceneComponent.K2_GetComponentLocation` (`self.Cube`))))
  ;[1 1 1] 前三块不生成障碍物
  (if (>= _returnvalue_x 1500.0)
    (`self.SpawnObstacles`)))

(event `self.Box.OnComponentBeginOverlap`
  (params (OverlappedComponent :type "PrimitiveComponent Object Reference") (OtherActor :type "Actor Object Reference") (OtherComp :type "PrimitiveComponent Object Reference") (OtherBodyIndex :type Integer) (bFromSweep :type Boolean) (SweepResult :type "HitResult Structure (by ref)"))
  ;[1 1 1] 产生后续砖块+加分
  (cast `CapsuleComponent` OtherComp)
  (cast `/Game/ThirdPersonBP/Blueprints/ThirdPersonCharacter` OtherActor)
  (bind _asthird_person_game_mode (cast `/Game/ThirdPersonBP/Blueprints/ThirdPersonGameMode` (`GameplayStatics.GetGameMode`)))
  (`/Game/ThirdPersonBP/Blueprints/ThirdPersonGameMode.SpawnTile` _asthird_person_game_mode)
  (`KismetSystemLibrary.Delay` 0.5)
  (bind _asthird_person_game_mode_2 (cast `/Game/ThirdPersonBP/Blueprints/ThirdPersonGameMode` (`GameplayStatics.GetGameMode`)))
  (set `/Game/ThirdPersonBP/Blueprints/ThirdPersonGameMode.CurrentPoints` (+ (`/Game/ThirdPersonBP/Blueprints/ThirdPersonGameMode.CurrentPoints` _asthird_person_game_mode_2) (`/Game/ThirdPersonBP/Blueprints/ThirdPersonGameMode.PointsMultiplier` _asthird_person_game_mode_2)) _asthird_person_game_mode_2)
  (`self.DestroySelf`))

(fn `DestroySelf`
  (bind _result (`BlueprintSetLibrary.Set_ToArray` (`self.ObstaclesList`)))
  (for _array_element _result
    (`/Engine/EditorBlueprintResources/StandardMacros.IsValid` _array_element
      (:`Is Valid`
        (`self.K2_DestroyActor` _array_element))))
  (`self.K2_DestroyActor`))

(fn `SpawnObstacles`
  (locals (Lanes :type "Array of ArrowComponent Object Reference") (rand :type "Float (double-precision)"))
  (set `local.Lanes` (`|MakeArray` (`self.Lane0`) (`self.Lane1`) (`self.Lane2`)))
  ;[1 1 1] Lane
  (for _index (range 3)
    (set `local.rand` (`KismetMathLibrary.RandomFloat`))
    (bind _keys (`BlueprintMapLibrary.Map_Keys` (`self.Obstacles`)))
    (for _array_element _keys
      (bind _output_get (set `local.rand` (- (`local.rand`) (`BlueprintMapLibrary.Map_Find` (`self.Obstacles`) _array_element))))
      (if (< _output_get 0.0)
        (bind _returnvalue (`|SpawnActorFromClass` _array_element (`SceneComponent.K2_GetComponentToWorld` (`|GetArrayItem` (`local.Lanes`) _index)) "Undefined" "OverrideRootScale" null null))
        (`/Engine/EditorBlueprintResources/StandardMacros.IsValid` _returnvalue
          (:`Is Valid`
            (bind _output_get_2 (set `self.ObstaclesList` (`self.ObstaclesList`)))
            (`BlueprintSetLibrary.Set_Add` _output_get_2 _returnvalue)
            (break)))))))

(fn `UserConstructionScript`)