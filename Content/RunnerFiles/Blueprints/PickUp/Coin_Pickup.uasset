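; Coin pickup for a runner game that adds coins to the player's total and can be pulled in by a magnet.
; Overlap between its mesh and the character's capsule adds CoinsMultiplier to the game mode's Coins, plays a 2D sound and destroys the coin.
; Entering MagnetBox with the magnet active starts a timeline that interpolates the coin toward just below the player's location, offset by a Slide track.
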(event `self.StaticMesh.OnComponentBeginOverlap`
  (params (OverlappedComponent :type "PrimitiveComponent Object Reference") (OtherActor :type "Actor Object Reference") (OtherComp :type "PrimitiveComponent Object Reference") (OtherBodyIndex :type Integer) (bFromSweep :type Boolean) (SweepResult :type "HitResult Structure (by ref)"))
  (cast `CapsuleComponent` OtherComp)
  (cast `/Game/ThirdPersonBP/Blueprints/ThirdPersonCharacter` OtherActor)
  (bind _asthird_person_game_mode (cast `/Game/ThirdPersonBP/Blueprints/ThirdPersonGameMode` (`GameplayStatics.GetGameMode`)))
  (set `/Game/ThirdPersonBP/Blueprints/ThirdPersonGameMode.Coins` (+ (`/Game/ThirdPersonBP/Blueprints/ThirdPersonGameMode.Coins` _asthird_person_game_mode) (`/Game/ThirdPersonBP/Blueprints/ThirdPersonGameMode.CoinsMultiplier` _asthird_person_game_mode)) _asthird_person_game_mode)
  (`GameplayStatics.SpawnSound2D` "/Game/RunnerFiles/SFX/Pickup_SFX.Pickup_SFX" 1.0 1.0 0.0 null)
  (`self.K2_DestroyActor`))

(event `self.MagnetBox.OnComponentBeginOverlap`
  (params (OverlappedComponent :type "PrimitiveComponent Object Reference") (OtherActor :type "Actor Object Reference") (OtherComp :type "PrimitiveComponent Object Reference") (OtherBodyIndex :type Integer) (bFromSweep :type Boolean) (SweepResult :type "HitResult Structure (by ref)"))
  (bind _asthird_person_character (cast `/Game/ThirdPersonBP/Blueprints/ThirdPersonCharacter` OtherActor))
  (if (`/Game/ThirdPersonBP/Blueprints/ThirdPersonCharacter.IsActiveMagnet` _asthird_person_character)
    (bind (_direction _slide) (`Timeline|Timeline_0` :!via `PlayFromStart`)
      (:`Update`
        (`self.K2_SetActorLocation` (+ _slide (`KismetMathLibrary.VInterpTo` (`self.K2_GetActorLocation`) (- (`self.K2_GetActorLocation` (`GameplayStatics.GetPlayerCharacter` 0)) (0.0 0.0 60.0)) (`GameplayStatics.GetWorldDeltaSeconds`) 10.0)))))))

(fn `UserConstructionScript`)